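; BP_Move is an actor that scrolls along the world X axis and loops back to the world origin.
; Each tick it offsets its root by Speed; once X drops to negative Distance or below, it prints that X and teleport-free resets to zero.
; Ticking is enabled on BeginPlay, and a leftover, unconnected Start node that would re-enable it never runs.
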(event EventBeginPlay
  (Actor|Tick|SetActorTickEnabled true))

(event Collision|EventActorBeginOverlap
  (params (OtherActor :type Actor%20Object%20Reference)))

(event EventTick
  (params (DeltaSeconds :type Float%20%28single-precision%29))
  (bind _defaultsceneroot (Variables|Default|GetDefaultSceneRoot))
  (bind _returnvalue (Transformation|GetWorldLocation _defaultsceneroot))
  (Transformation|AddWorldOffset _defaultsceneroot (Math|Vector|MakeVector (Variables|Default|GetSpeed) 0.0 0.0) false false)
  (if (<= (.x _returnvalue) (- 0.0 (Variables|Default|GetDistance)))
    (Development|PrintString (Utilities|String|ToString(Float) (.x _returnvalue)))
    (Transformation|SetWorldLocation (Variables|Default|GetDefaultSceneRoot) "0, 0, 0" false false)))

(fn ConstructionScript)