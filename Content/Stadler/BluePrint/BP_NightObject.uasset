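; BP_NightObject is a placeable actor whose static mesh swaps between a day and a night version.
; A SetDay event takes a day flag and sets the mesh component to MeshDay or MeshNight, skipping the swap if that mesh is not assigned.
; The construction script applies the day mesh, so it shows by default.
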(event EventBeginPlay)

(event Collision|EventActorBeginOverlap
  (params (OtherActor :type Actor%20Object%20Reference)))

(event EventTick
  (params (DeltaSeconds :type Float%20%28single-precision%29)))

(event EventSetDay
  (params (Day :type Boolean))
  (bind _mesh_day (Variables|Default|GetMesh_Day))
  (bind _mesh_night (Variables|Default|GetMesh_Night))
  (if Day
    (Utilities|IsValid _mesh_day
      (:Is%20Valid
        (Components|StaticMesh|SetStaticMesh (Variables|Default|GetMesh) _mesh_day)))
    (else
      (Utilities|IsValid _mesh_night
        (:Is%20Valid
          (Components|StaticMesh|SetStaticMesh (Variables|Default|GetMesh) _mesh_night))))))

(fn ConstructionScript
  (bind _mesh_day (Variables|Default|GetMesh_Day))
  (Utilities|IsValid _mesh_day
    (:Is%20Valid
      (Components|StaticMesh|SetStaticMesh (Variables|Default|GetMesh) _mesh_day))))