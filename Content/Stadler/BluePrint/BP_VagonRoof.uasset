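; BP_VagonRoof is a wagon roof actor that lifts away and hides when its wagon is the selected section.
; BeginPlay caches the default location and turns HideLoc from an offset into a target position.
; SetNewState plays a timeline that lerps between them, hiding the mesh when fully lifted; General state or another wagon's selection shows it and reverses the move.
; The construction script applies an optional Mesh override.
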(event EventBeginPlay
  (bind _output_get (Variables|Default|SetDefaultLoc (Transformation|GetActorLocation)))
  (Variables|Default|SetHideLoc (+ _output_get (Variables|Default|GetHideLoc))))

(event Collision|EventActorBeginOverlap
  (params (OtherActor :type Actor%20Object%20Reference)))

(event EventTick
  (params (DeltaSeconds :type Float%20%28single-precision%29)))

(event EventSetNewState
  (params (NewState :type E_TrainState%20Enum :default "NewEnumerator0") (SectionSelect :type BP%20Touch%20Vagon%20Object%20Reference) (FlatSelect :type BP%20Touch%20Coupe%20Object%20Reference) (SelectGroup :type Integer) (IsChange :type Boolean))
  (switch Utilities|FlowControl|Switch|SwitchonE_TrainState NewState
    (:NewEnumerator0
      (Rendering|SetVisibility (Variables|Default|GetSM_VagonRoof) true false :!label _label)
      (bind _lift (Timeline|Timeline Reverse)
        (:Update
          (Transformation|SetActorLocation (Math|Vector|Lerp(Vector) (Variables|Default|GetDefaultLoc) (Variables|Default|GetHideLoc) _lift) false false))
        (:Finished
          (Rendering|SetVisibility (Variables|Default|GetSM_VagonRoof) (< _lift 1.0) false))))
    (:NewEnumerator2
      (if (== (Variables|Default|GetVagon) (Variables|/Game/Core/BP_TouchVagon.BP_TouchVagon_C|GetVagon SectionSelect))
        (Timeline|Timeline Play)
        (else
          (goto _label))))))

(fn ConstructionScript
  (bind _mesh (Variables|Default|GetMesh))
  (Utilities|IsValid _mesh
    (:Is%20Valid
      (Components|StaticMesh|SetStaticMesh (Variables|Default|GetSM_VagonRoof) _mesh))))