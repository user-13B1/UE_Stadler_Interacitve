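; BP_HideWall is a train car wall actor whose visibility toggles by side for the current car or section.
; HideWall checks either a section state or the current car number against Vagon, then sets visibility from an IsRight comparison.
; Non-matching cars are shown, while non-matching section states leave visibility unchanged; ShowWall always reveals the wall.
; Visibility propagates from the root to children, and the construction script applies an optional mesh override.
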(event EventBeginPlay)

(event Collision|EventActorBeginOverlap
  (params (OtherActor :type Actor%20Object%20Reference)))

(event EventTick
  (params (DeltaSeconds :type Float%20%28single-precision%29)))

(event EventHideWall
  (params (IsHide :type Boolean) (IsRight :type Boolean))
  (if (Variables|Default|GetIsSection)
    (bind _currentscenastate (CallFunction|GetCurrState))
    (if (Utilities|Enum|Equal(Enum) _currentscenastate "NewEnumerator1")
      (Rendering|SetVisibility (Variables|Default|GetDefaultSceneRoot) (== IsRight (Variables|Default|GetIsRight)) true :!label _label))
    (else
      (bind _currvagonnum (CallFunction|GetCurrVagonNum))
      (if (== _currvagonnum (Variables|Default|GetVagon))
        (goto _label)
        (else
          (Rendering|SetVisibility (Variables|Default|GetDefaultSceneRoot) true true))))))

(event EventShowWall
  (Rendering|SetVisibility (Variables|Default|GetDefaultSceneRoot) true true))

(fn ConstructionScript
  (bind _mesh (Variables|Default|GetMesh))
  (Utilities|IsValid _mesh
    (:Is%20Valid
      (Components|StaticMesh|SetStaticMesh (Variables|Default|GetSM_TrainСar_Compartment-01_Wall_Back) _mesh))))