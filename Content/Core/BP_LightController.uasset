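; Level light controller that switches movable point and rect lights on at night and off by day.
; Lights start hidden on BeginPlay, and the NightIsComing event toggles them through SetPointLight and SetRectLight.
; Both functions scan all actors of their class, skipping those tagged DayLight, and set component visibility.
; The construction script applies the same toggle from the Debug flag, showing lights when it is true.
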(event EventBeginPlay
  (CallFunction|SetPointLight true)
  (CallFunction|SetRectLight true))

(event Collision|EventActorBeginOverlap
  (params (OtherActor :type Actor%20Object%20Reference)))

(event EventTick
  (params (DeltaSeconds :type Float%20%28single-precision%29)))

(event EventNightIsComing
  (params (IsNight :type Boolean))
  (bind _returnvalue (not IsNight))
  (Utilities|FlowControl|Sequence
    (:then_0
      (CallFunction|SetPointLight _returnvalue))
    (:then_1
      (CallFunction|SetRectLight _returnvalue))))

(fn ConstructionScript
  (bind _debug (Variables|Default|GetDebug))
  (bind _returnvalue (not _debug))
  (CallFunction|SetPointLight _returnvalue)
  (CallFunction|SetRectLight _returnvalue))

(fn SetPointLight
  (params (NewHidden :type Boolean))
  (bind _outactors (Actor|GetAllActorsOfClass "/Script/Engine.PointLight"))
  (for _array_element _outactors
    (switch Utilities|FlowControl|Switch|SwitchonEComponentMobility (Variables|/Script/Engine.SceneComponent|GetMobility (Variables|/Script/Engine.PointLight|GetPointLightComponent _array_element))
      (:Movable
        (if (not (Actor|ActorHasTag _array_element "DayLight"))
          (Development|SetHiddeninGame (Variables|/Script/Engine.PointLight|GetPointLightComponent _array_element) NewHidden false)
          (Rendering|SetVisibility (Variables|/Script/Engine.PointLight|GetPointLightComponent _array_element) (not NewHidden) false))))))

(fn SetRectLight
  (params (NewHidden :type Boolean))
  (bind _outactors (Actor|GetAllActorsOfClass "/Script/Engine.RectLight"))
  (for _array_element _outactors
    (switch Utilities|FlowControl|Switch|SwitchonEComponentMobility (Variables|/Script/Engine.SceneComponent|GetMobility (Variables|/Script/Engine.Actor|GetRootComponent _array_element))
      (:Movable
        (if (not (Actor|ActorHasTag _array_element "DayLight"))
          (Development|SetHiddeninGame (Variables|/Script/Engine.Actor|GetRootComponent _array_element) NewHidden false)
          (Rendering|SetVisibility (Variables|/Script/Engine.Actor|GetRootComponent _array_element) (not NewHidden) false))))))