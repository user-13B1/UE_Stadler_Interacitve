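; BP_HideHouse is a house actor that hides its mesh while something overlaps it.
; The construction script applies the House mesh to HouseMesh and, if DopMesh is also set, adds a second auto-attached static mesh component for it.
; HouseMesh overlap begin and end events toggle visibility with propagation to child components, without filtering the overlapping actor or counting overlaps.
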(event OnComponentBeginOverlap(HouseMesh)
  (params (OverlappedComponent :type Primitive%20Component%20Object%20Reference) (OtherActor :type Actor%20Object%20Reference) (OtherComp :type Primitive%20Component%20Object%20Reference) (OtherBodyIndex :type Integer) (bFromSweep :type Boolean) (SweepResult :type Hit%20Result%20Structure%20%28by%20ref%29))
  (Rendering|SetVisibility (Variables|Default|GetHouseMesh) false true))

(event OnComponentEndOverlap(HouseMesh)
  (params (OverlappedComponent :type Primitive%20Component%20Object%20Reference) (OtherActor :type Actor%20Object%20Reference) (OtherComp :type Primitive%20Component%20Object%20Reference) (OtherBodyIndex :type Integer))
  (Rendering|SetVisibility (Variables|Default|GetHouseMesh) true true))

(event EventBeginPlay)

(event Collision|EventActorBeginOverlap
  (params (OtherActor :type Actor%20Object%20Reference)))

(event EventTick
  (params (DeltaSeconds :type Float%20%28single-precision%29)))

(fn ConstructionScript
  (bind _house (Variables|Default|GetHouse))
  (bind _dopmesh (Variables|Default|GetDopMesh))
  (Utilities|IsValid _house
    (:Is%20Valid
      (Components|StaticMesh|SetStaticMesh (Variables|Default|GetHouseMesh) _house)
      (Utilities|IsValid _dopmesh
        (:Is%20Valid
          (bind _returnvalue (AddComponent|AddStaticMeshComponent false))
          (bind _output_get (LocalVariables|SetStaticDopMesh _returnvalue))
          (Components|StaticMesh|SetStaticMesh _output_get _dopmesh))))))