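; Highlight mesh actor that briefly flickers when its House and Part match the section or flat selected through SetNewState.
; It stays hidden until matched: Vagon state plays a PowerLight material flicker, while Coupe state also lerps the actor toward a point below before resetting it.
; One-shot flags stop repeat flickers until the selection or state resets them, and a Debug flag controls visibility in construction.
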(event Custom|FlickSection
  (params (House :type Integer) (Part :type Integer))
  ;[1 1 1] FlickSection
  (Variables|Default|SetOneFlickFlatFlag false)
  (if (Math|Boolean|ANDBoolean (== House (Variables|Default|GetHouse)) (== Part (Variables|Default|GetPart)) (not (Variables|Default|GetOneFlickSectionFlag)))
    (Variables|Default|SetOneFlickSectionFlag true)
    (Development|SetHiddeninGame (Variables|Debug|GetStaticMeshComponent) false false)
    (bind _flicklight (Timeline|FlickB PlayFromStart)
      (:Update
        (Rendering|Material|SetScalarParameterValueonMaterials (Variables|Debug|GetStaticMeshComponent) "PowerLight" _flicklight))
      (:Finished
        (Development|SetHiddeninGame (Variables|Debug|GetStaticMeshComponent) true false)))
    (else
      (Variables|Default|SetOneFlickSectionFlag false))))

(event Custom|FlickFlatSelect
  (params (House :type Integer) (Part :type Integer))
  (if (Math|Boolean|ANDBoolean (== House (Variables|Default|GetHouse)) (== Part (Variables|Default|GetPart)) (not (Variables|Default|GetOneFlickFlatFlag)))
    (Variables|Default|SetOneFlickFlatFlag true)
    (Development|SetHiddeninGame (Variables|Debug|GetStaticMeshComponent) false false)
    (bind (_direction _flicklight _lift) (Timeline|FlickA PlayFromStart)
      (:Update
        (Rendering|Material|SetScalarParameterValueonMaterials (Variables|Debug|GetStaticMeshComponent) "PowerLight" _flicklight)
        (Transformation|SetActorLocation self (Math|Vector|Lerp(Vector) (Variables|Default|GetStartLacation) (Variables|Default|GetHideLocation) _lift) false true))
      (:Finished
        (Development|SetHiddeninGame (Variables|Debug|GetStaticMeshComponent) true false)
        (Transformation|SetActorLocation (Variables|Default|GetStartLacation) false true)))))

(event EventBeginPlay
  (bind _self self)
  (bind _returnvalue (Transformation|GetActorLocation _self))
  (bind (_x _y _z) (Math|Vector|BreakVector _returnvalue))
  (Rendering|SetVisibility (Variables|Debug|GetStaticMeshComponent) true false)
  (Development|SetHiddeninGame (Variables|Debug|GetStaticMeshComponent) true false)
  (Variables|Default|SetStartLacation _returnvalue)
  (Variables|Default|SetHideLocation (Math|Vector|MakeVector _x _y (- _z 2e+03))))

(event EventSetNewState
  (params (NewState :type E_TrainState%20Enum :default "NewEnumerator0") (SectionSelect :type BP%20Touch%20Vagon%20Object%20Reference) (FlatSelect :type BP%20Touch%20Coupe%20Object%20Reference) (SelectGroup :type Integer) (IsChange :type Boolean))
  (switch Utilities|FlowControl|Switch|SwitchonE_TrainState NewState
    (:NewEnumerator0
      (Variables|Default|SetOneFlickFlatFlag false)
      (Variables|Default|SetOneFlickSectionFlag false))
    (:NewEnumerator2
      (CallFunction|FlickSection (Variables|/Game/Core/BP_TouchVagon.BP_TouchVagon_C|GetVagon SectionSelect) (Variables|/Game/Core/BP_TouchVagon.BP_TouchVagon_C|GetTrain SectionSelect)))
    (:NewEnumerator1
      (CallFunction|FlickFlatSelect (Variables|/Game/Core/BP_TouchCoupe.BP_TouchCoupe_C|GetVagon FlatSelect) (Variables|/Game/Core/BP_TouchCoupe.BP_TouchCoupe_C|GetTrain FlatSelect)))))

(fn ConstructionScript
  (Rendering|SetVisibility (Variables|Debug|GetStaticMeshComponent) (Variables|Default|GetDebug) false))