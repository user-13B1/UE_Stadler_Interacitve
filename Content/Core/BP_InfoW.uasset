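; Tappable info marker for an architectural scene that yaw-rotates toward the pawn camera while rendered.
; Visibility and touch collision follow scene state, with one state also matching the selected flat's house, part and floor.
; A timed Gate accepts only short taps, which, unless the game mode blocks, broadcast textures and texts to every VIR_ScenaState_Interface widget and actor.
; Tapping also flashes the marker and dims it until a timer restores its lit material.
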(event OnInputTouchEnd(Sphere)
  (params (FingerIndex :type ETouchIndex%20Enum :default "Touch1") (TouchedComponent :type Primitive%20Component%20Object%20Reference))
  (Utilities|FlowControl|Gate true
    (:Exit
      (if (not (Default|IsBlock (Variables|Default|GetGame%20Mode)))
        (Rendering|Material|SetMaterial (Variables|Debug|GetStaticMeshComponent) 0 "/Game/Collection/Materials/Xray/MI_GeoTag_Flick.MI_GeoTag_Flick")
        (Utilities|Time|SetTimerbyFunctionName 0 "SetStartDefaultMaterial" 1.2e+02)
        (Utilities|FlowControl|Delay 0.1)
        (Rendering|Material|SetMaterial (Variables|Debug|GetStaticMeshComponent) 0 "/Game/Collection/Materials/Xray/MI_GeoTag_Off.MI_GeoTag_Off")
        (Utilities|FlowControl|Sequence
          (:then_0
            (bind _foundwidgets (Class|WidgetBlueprintLibrary|GetAllWidgetswithInterface "/Game/Core/VIR_ScenaState_Interface.VIR_ScenaState_Interface_C" false))
            (for _array_element _foundwidgets
              (Class|VIRScenaStateInterface|ShowInfoWidget(Message) _array_element true (Variables|Default|GetTexture_Array) (Variables|Default|GetIsShowText) (Variables|Default|GetTitle1) (Variables|Default|GetText1) (Variables|Default|GetTitle2) (Variables|Default|GetText2) (Variables|Default|GetTitle3) (Variables|Default|GetText3))))
          (:then_1
            (bind _outactors (Actor|GetAllActorswithInterface "/Game/Core/VIR_ScenaState_Interface.VIR_ScenaState_Interface_C"))
            (for _array_element_2 _outactors
              (Class|VIRScenaStateInterface|ShowInfoWidget(Message) _array_element_2 true (Variables|Default|GetTexture_Array) (Variables|Default|GetIsShowText) (Variables|Default|GetTitle1) (Variables|Default|GetText1) (Variables|Default|GetTitle2) (Variables|Default|GetText2) (Variables|Default|GetTitle3) (Variables|Default|GetText3)))))))))

(event OnInputTouchBegin(Sphere)
  (params (FingerIndex :type ETouchIndex%20Enum :default "Touch1") (TouchedComponent :type Primitive%20Component%20Object%20Reference))
  (Utilities|FlowControl|Sequence
    (:then_0
      (Utilities|FlowControl|Gate true) ; enters at Open
    )
    (:then_1
      (Utilities|FlowControl|Delay 0.3)
      (Utilities|FlowControl|Gate true) ; enters at Close
    )))

(event Custom|Touch
  (if (not (Default|IsBlock (Variables|Default|GetGame%20Mode)))
    (Rendering|Material|SetMaterial (Variables|Debug|GetStaticMeshComponent) 0 "/Game/Collection/Materials/Xray/MI_GeoTag_Flick.MI_GeoTag_Flick")
    (Utilities|Time|SetTimerbyFunctionName 0 "SetStartDefaultMaterial" 1.2e+02)
    (Utilities|FlowControl|Delay 0.1)
    (Rendering|Material|SetMaterial (Variables|Debug|GetStaticMeshComponent) 0 "/Game/Collection/Materials/Xray/MI_GeoTag_Off.MI_GeoTag_Off")
    (Utilities|FlowControl|Sequence
      (:then_0
        (bind _foundwidgets (Class|WidgetBlueprintLibrary|GetAllWidgetswithInterface "/Game/Core/VIR_ScenaState_Interface.VIR_ScenaState_Interface_C" false))
        (for _array_element _foundwidgets
          (Class|VIRScenaStateInterface|ShowInfoWidget(Message) _array_element true (Variables|Default|GetTexture_Array) (Variables|Default|GetIsShowText) (Variables|Default|GetTitle1) (Variables|Default|GetText1) (Variables|Default|GetTitle2) (Variables|Default|GetText2) (Variables|Default|GetTitle3) (Variables|Default|GetText3))))
      (:then_1
        (bind _outactors (Actor|GetAllActorswithInterface "/Game/Core/VIR_ScenaState_Interface.VIR_ScenaState_Interface_C"))
        (for _array_element_2 _outactors
          (Class|VIRScenaStateInterface|ShowInfoWidget(Message) _array_element_2 true (Variables|Default|GetTexture_Array) (Variables|Default|GetIsShowText) (Variables|Default|GetTitle1) (Variables|Default|GetText1) (Variables|Default|GetTitle2) (Variables|Default|GetText2) (Variables|Default|GetTitle3) (Variables|Default|GetText3)))))))

(event EventBeginPlay
  (bind _returnvalue (Game|Player|GetPlayerPawn 0))
  ;[1 1 1] Comment
  (bind _gamemode (CallFunction|GetArchGameMode))
  (Variables|Default|SetGame%20Mode _gamemode)
  (CallFunction|Show (Utilities|Enum|Equal(Enum) "NewEnumerator0" (Variables|Default|GetState)))
  (Utilities|IsValid _returnvalue
    (:Is%20Valid
      (bind _asarch_pawn (Utilities|Casting|CastToArch_Pawn _returnvalue)
        (:then
          (Variables|Default|SetAs%20Arch%20Pawn _asarch_pawn))
        (:CastFailed
          (Development|PrintString "No Valid Arch Pawn" :!label _label)
          (Variables|Default|SetEnable false))))
    (:Is%20Not%20Valid
      (goto _label))))

(event Collision|EventActorBeginOverlap
  (params (OtherActor :type Actor%20Object%20Reference)))

(event EventTick
  (params (DeltaSeconds :type Float%20%28single-precision%29))
  ;[1 1 1] RotateToUserCamera
  (if (Variables|Default|GetEnable)
    (if (Class|PrimitiveComponent|WasRecentlyRendered (Variables|Debug|GetStaticMeshComponent) 0.2)
      (Transformation|SetWorldRotation (Variables|Debug|GetStaticMeshComponent) (Math|Rotator|MakeRotator 0.0 0.0 (+ (.yaw (Math|Rotator|FindLookatRotation (Transformation|GetWorldLocation (Variables|Debug|GetStaticMeshComponent)) (Default|GetCameraLoaction (Variables|Default|GetAs%20Arch%20Pawn)))) -9e+01)) false false))))

(event EventSetNewState
  (params (NewState :type E_TrainState%20Enum :default "NewEnumerator0") (SectionSelect :type BP%20Touch%20Vagon%20Object%20Reference) (FlatSelect :type BP%20Touch%20Coupe%20Object%20Reference) (SelectGroup :type Integer) (IsChange :type Boolean))
  ;[1 1 1] Comment
  (CallFunction|IfShow (Utilities|Enum|Equal(Enum) NewState (Variables|Default|GetState)) FlatSelect))

(event EventSetVisibleGameInterface
  (params (Value :type Boolean))
  (CallFunction|Show Value))

(fn ConstructionScript
  (if (not (Variables|Default|GetIsImage))
    (Components|StaticMesh|SetStaticMesh (Variables|Debug|GetStaticMeshComponent) "/Game/Akbulak/Widget/InfoWidget/SM_InfoLogo.SM_InfoLogo")
    (else
      (Components|StaticMesh|SetStaticMesh (Variables|Debug|GetStaticMeshComponent) "/Game/Akbulak/Widget/InfoWidget/SM_InfoLogo_image.SM_InfoLogo_image"))))

(fn IfShow
  (params (Value :type Boolean) (Flat :type BP%20Touch%20Coupe%20Object%20Reference))
  (if (Utilities|Enum|NotEqual(Enum) (Variables|Default|GetState) "NewEnumerator1")
    (CallFunction|Show Value)
    (elif Value
      (Utilities|IsValid Flat
        (:Is%20Valid
          (CallFunction|Show (Math|Boolean|ANDBoolean (== (Variables|Default|Gethouse) (Variables|/Game/Core/BP_TouchCoupe.BP_TouchCoupe_C|GetVagon Flat)) (== (Variables|Default|Getpart) (Variables|/Game/Core/BP_TouchCoupe.BP_TouchCoupe_C|GetTrain Flat)) (== (Variables|/Game/Core/BP_TouchCoupe.BP_TouchCoupe_C|GetFloor Flat) (Variables|Default|Getfloor))))))
      (else
        (CallFunction|Show false)))))

(fn EquilFlat
  (params (Flat :type BP%20Touch%20Coupe%20Object%20Reference))
  (return (Math|Boolean|ANDBoolean (== (Variables|/Game/Core/BP_TouchCoupe.BP_TouchCoupe_C|GetVagon Flat) (Variables|Default|Gethouse)) (== (Variables|/Game/Core/BP_TouchCoupe.BP_TouchCoupe_C|GetTrain Flat) (Variables|Default|Getpart)) (== (Variables|/Game/Core/BP_TouchCoupe.BP_TouchCoupe_C|GetFloor Flat) (Variables|Default|Getfloor)))))

(fn Show
  (params (Value :type Boolean))
  (bind _sphere (Variables|Default|GetSphere))
  (Development|SetHiddeninGame (Variables|Debug|GetStaticMeshComponent) (not Value) false)
  (if Value
    (Collision|SetCollisionEnabled _sphere "QueryAndPhysics")
    (else
      (Collision|SetCollisionEnabled _sphere "NoCollision"))))

(fn SetStartDefaultMaterial
  (Rendering|Material|SetMaterial (Variables|Debug|GetStaticMeshComponent) 0 "/Game/Collection/Materials/Xray/MI_GeoTag_Light.MI_GeoTag_Light"))