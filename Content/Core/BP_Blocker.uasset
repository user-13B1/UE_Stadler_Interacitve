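; BP_Blocker is an actor that runs an online license check and stops the game if it fails.
; Thirty seconds after BeginPlay, it sends a GET request with a random CodeOut key to a hardcoded balakir.ru PHP endpoint.
; If the request fails or the response is not in CodeIn, BlockGame shows a root-widget error, when that widget is valid, and calls StopGameErrorLicense on the ArchGameMode.
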(event EventBeginPlay
  (Utilities|FlowControl|Delay 3e+01)
  (bind _returnvalue (Class|LowEntryHttpRequestLibrary|RequestCreate))
  (bind _output_get (Variables|Default|SetRequset _returnvalue))
  (Class|LowEntryHttpRequest|SetUrl _output_get "GET" "https://balakir.ru/telegram/modhouse/key.php")
  (Class|LowEntryHttpRequest|SetUrlParameter (Variables|Default|GetRequset) "keyUe4" (CallFunction|GetKey))
  (bind _response (Class|LowEntryHttpRequest|ExecuteRequest (Variables|Default|GetRequset)))
  (Class|LowEntryHttpRequestResponse|WasSuccessful _response
    (:Success
      (if (!= (Utilities|Array|FindItem (Variables|Default|GetCodeIn) (Class|LowEntryHttpRequestResponse|GetContentasString _response)) -1)
        (Development|PrintString "Server connect.")
        (else
          (CallFunction|BlockGame))))
    (:Failed
      (Development|PrintString "Error connect")
      (CallFunction|BlockGame))))

(event Collision|EventActorBeginOverlap
  (params (OtherActor :type Actor%20Object%20Reference)))

(event EventTick
  (params (DeltaSeconds :type Float%20%28single-precision%29)))

(fn ConstructionScript)

(fn BlockGame
  (Development|PrintString "Error code server.")
  (bind (_widget _isvalid) (CallFunction|GetRootWidget))
  (if _isvalid
    (Default|ShowErrorMessage _widget))
  (bind _gamemode (CallFunction|GetArchGameMode))
  (Default|StopGameErrorLicense _gamemode))

(fn GetKey
  (bind _codeout (Variables|Default|GetCodeOut))
  (return (Utilities|Array|Get(acopy) _codeout (Math|Random|RandomIntegerinRange 0 (Utilities|Array|LastIndex _codeout)))))