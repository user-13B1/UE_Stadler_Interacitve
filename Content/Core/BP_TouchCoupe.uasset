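; BP_TouchCoupe is a touchable hotspot for selecting a train compartment (Coupe) within a car (Vagon).
; A Delay-timed double tap on TouchMesh flashes it and broadcasts the Coupe state when ArchGameMode is free.
; SetNewState toggles visibility and collision by matching car or compartment, spawning a border mesh component on the selected one.
; Separate light and block flags control backlight highlighting, and Debug exposes the collision mesh.
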(event OnInputTouchBegin(TouchMesh)
  (params (FingerIndex :type ETouchIndex%20Enum :default "Touch1") (TouchedComponent :type Primitive%20Component%20Object%20Reference))
  ;[1 1 1] Touch
  (switch Utilities|FlowControl|Switch|SwitchonETouchIndex FingerIndex
    (:Touch1
      (if (and (Variables|Flags|GetSuitableToTouch) (not (Variables|Flags|GetIsSelected)))
        (if (not (Variables|Flags|GetIsTouchOne))
          (Variables|Default|SetButtonDribbleBlock true)
          (Variables|Flags|SetIsTouchOne true)
          (Utilities|FlowControl|Delay 0.6)
          (Variables|Flags|SetIsTouchOne false)
          (elif (and (not (Variables|Flags|GetIsTouchTwo)) (not (Variables|Default|GetButtonDribbleBlock)))
            (Variables|Flags|SetIsTouchTwo true)
            (Utilities|FlowControl|Delay 0.2)
            (Variables|Flags|SetIsTouchTwo false)
            (else
              (Development|PrintString "Dribble block" true true "(R=1.000000,G=0.000000,B=0.007234,A=1.000000)" 3.0))))))
    (:Touch2
      (Development|PrintString "Touch two fingre. " :!label _label))
    (:Touch3
      (goto _label))))

(event OnInputTouchEnd(TouchMesh)
  (params (FingerIndex :type ETouchIndex%20Enum :default "Touch1") (TouchedComponent :type Primitive%20Component%20Object%20Reference))
  ;[1 1 1] Touch
  (if (and (Variables|Flags|GetIsTouchOne) (not (Variables|Flags|GetIsTouchTwo)))
    (Utilities|FlowControl|Delay 0.05)
    (Variables|Default|SetButtonDribbleBlock false)
    (elif (Math|Boolean|ANDBoolean (Variables|Flags|GetIsTouchTwo) (Variables|Flags|GetSuitableToTouch) (Default|IsFree (Variables|Links|GetArchGameMode)))
      (CallFunction|FlickMesh)
      (CallFunction|SendAllNewState "NewEnumerator1" 0 self)
      (else
        (Development|PrintString "Block select touch" true true "(R=1.000000,G=0.000000,B=0.007234,A=1.000000)" 3.0)))))

(event Custom|SetStateVagon
  (params (Section%20Select :type BP%20Touch%20Vagon%20Object%20Reference))
  ;[1 1 1] Set Section State
  (CallFunction|Deselect)
  (if (== (Variables|Info|GetVagon) (Variables|/Game/Core/BP_TouchVagon.BP_TouchVagon_C|GetVagon Section%20Select))
    (CallFunction|ShowTouch)
    (else
      (CallFunction|HideTouch))))

(event Custom|FlickMesh
  ;[1 1 1] FlickMesh
  (Development|SetHiddeninGame (Variables|Default|GetTouchMesh) false false)
  (Utilities|FlowControl|Delay 0.1)
  (Development|SetHiddeninGame (Variables|Default|GetTouchMesh) true false))

(event Custom|SetStateFlat
  (params (CurrentFlatSelect :type BP%20Touch%20Coupe%20Object%20Reference))
  ;[1 1 1] Comment
  (Utilities|FlowControl|Sequence
    (:then_0
      (if (== self CurrentFlatSelect)
        (CallFunction|SelectThisFlat)
        (else
          (CallFunction|Deselect))))
    (:then_1
      (if (and (== (Variables|BP_TouchCoupe_C|GetVagon CurrentFlatSelect) (Variables|Info|GetVagon)) (== (Variables|Info|GetTrain) (Variables|BP_TouchCoupe_C|GetTrain CurrentFlatSelect)))
        (if (Variables|Flags|GetIsHide)
          (CallFunction|ShowTouch))))
    (:then_2
      (CallFunction|Lighton false))))

(event Custom|SelectThisFlat
  ;[1 1 1] Select
  (if (not (Variables|Flags|GetIsSelected))
    (Variables|Flags|SetIsSelected true)
    (Utilities|IsValid (Variables|Border|GetBorderMesh)
      (:Is%20Valid
        (bind _returnvalue (AddComponent|AddStaticMeshComponent false))
        (bind _output_get (Variables|Border|SetBorderComponent _returnvalue))
        (Components|StaticMesh|SetStaticMesh _output_get (Variables|Border|GetBorderMesh))))))

(event Custom|Deselect
  ;[1 1 1] Deselect
  (if (Variables|Flags|GetIsSelected)
    (Variables|Flags|SetIsSelected false)
    (Utilities|IsValid (Variables|Border|GetBorderMesh)
      (:Is%20Valid
        (Components|DestroyComponent (Variables|Border|GetBorderComponent))))))

(event EventBeginPlay
  ;[1 1 1] Start
  (CallFunction|StartSetting)
  (Development|SetHiddeninGame (Variables|Default|GetTouchMesh) true false))

(event EventSetNewState
  (params (NewState :type E_TrainState%20Enum :default "NewEnumerator0") (SectionSelect :type BP%20Touch%20Vagon%20Object%20Reference) (FlatSelect :type BP%20Touch%20Coupe%20Object%20Reference) (SelectGroup :type Integer) (IsChange :type Boolean))
  ;[1 1 1] SetState
  (switch Utilities|FlowControl|Switch|SwitchonE_TrainState NewState
    (:NewEnumerator0
      (CallFunction|HideTouch)
      (CallFunction|Deselect)
      (CallFunction|Lighton false))
    (:NewEnumerator2
      (CallFunction|SetStateVagon SectionSelect))
    (:NewEnumerator1
      (CallFunction|SetStateFlat FlatSelect))))

(event EventShowBacklightSelectHouse
  (params (Show :type Boolean))
  ;[1 1 1] BackLight
  (if Show
    (Variables|Default|SetIsBlockLight false)
    (if (Variables|Default|GetIsLightOn)
      (Development|SetHiddeninGame (Variables|Default|GetTouchMesh) false false))
    (else
      (Variables|Default|SetIsBlockLight true)
      (if (Variables|Default|GetIsLightOn)
        (Development|SetHiddeninGame (Variables|Default|GetTouchMesh) true false)))))

(fn ConstructionScript
  (bind _meshcollision (Variables|Default|GetMeshCollision))
  (Utilities|IsValid _meshcollision
    (:Is%20Valid
      (Components|StaticMesh|SetStaticMesh (Variables|Default|GetTouchMesh) _meshcollision)
      (if (Variables|Default|GetDebug)
        (Rendering|SetVisibility (Variables|Default|GetTouchMesh) true false)
        (else
          (Rendering|SetVisibility (Variables|Default|GetTouchMesh) false false))))))

(fn StartSetting
  (if (Math|Boolean|ANDBoolean (!= (Variables|Info|GetSection) 0) (!= (Variables|Info|GetVagon) 0) (!= (Variables|Info|GetFloor) 0))
    (bind _gamemode (CallFunction|GetArchGameMode))
    (Variables|Links|SetArchGameMode _gamemode)
    (CallFunction|HideTouch)
    (else
      (Development|PrintString "BP_tocherFlat - data not set." true true "(R=1.000000,G=0.000000,B=0.037674,A=1.000000)"))))

(fn ShowTouch
  (if (Variables|Flags|GetIsHide)
    (Collision|SetCollisionEnabled (Variables|Default|GetTouchMesh) "QueryAndPhysics")
    (Variables|Flags|SetSuitableToTouch true)
    (Variables|Flags|SetIsHide false)
    (Development|SetHiddeninGame (Variables|Default|GetTouchMesh) (not (Variables|Default|GetDebug)) false)))

(fn HideTouch
  (if (not (Variables|Flags|GetIsHide))
    (Collision|SetCollisionEnabled (Variables|Default|GetTouchMesh) "NoCollision")
    (Variables|Flags|SetSuitableToTouch false)
    (Variables|Flags|SetIsHide true)
    (Development|SetHiddeninGame (Variables|Default|GetTouchMesh) true false)))

(fn Lighton
  (params (IsLight :type Boolean))
  (bind _touchmesh (Variables|Default|GetTouchMesh))
  (bind _isblocklight (Variables|Default|GetIsBlockLight))
  (bind _returnvalue (not _isblocklight))
  (if IsLight
    (if (not (Variables|Default|GetIsLightOn))
      (Variables|Default|SetIsLightOn true)
      (if _returnvalue
        (Development|SetHiddeninGame _touchmesh false false)))
    (elif (Variables|Default|GetIsLightOn)
      (Variables|Default|SetIsLightOn false)
      (if _returnvalue
        (Development|SetHiddeninGame _touchmesh true false)))))

(fn GetPanorama
  (return (Variables|Panorams|GetData%20Table)))