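; BP_Light_Mesh is a mesh actor that shows or hides its static mesh according to time of day and season.
; SetDayTime shows it during the night window unless AlwaysLight is set; season events override that flag and visibility, with Summer clearing both.
; These changes pass through SetNewVisibility, which ignores them during a five-second freeze after BeginPlay hides the mesh.
; The construction script applies the Debug flag as visibility, and Hide bypasses the freeze.
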(event EventBeginPlay
  (Rendering|SetVisibility (Variables|Debug|GetStaticMeshComponent) false false)
  (Variables|Default|SetFreeze true)
  (Utilities|FlowControl|Delay 5.0)
  (Variables|Default|SetFreeze false))

(event Collision|EventActorBeginOverlap
  (params (OtherActor :type Actor%20Object%20Reference)))

(event EventTick
  (params (DeltaSeconds :type Float%20%28single-precision%29)))

(event EventAutumn
  (bind _autumlight (Variables|Default|GetAutumLight))
  (Variables|Default|SetAlwaysLight _autumlight)
  (CallFunction|SetNewVisibility _autumlight))

(event EventSummer
  (Variables|Default|SetAlwaysLight false)
  (CallFunction|SetNewVisibility false))

(event EventSetDayTime
  (params (Time :type Float%20%28single-precision%29))
  (if (not (Variables|Default|GetAlwaysLight))
    (CallFunction|SetNewVisibility (or (Math|Float|InRange(Float) Time 0.0 (Variables|Default|GetEndLightTime)) (Math|Float|InRange(Float) Time (Variables|Default|GetStartLightTime) 24.0)))))

(event EventWinter
  (bind _winterlight (Variables|Default|GetWinterLight))
  (Variables|Default|SetAlwaysLight _winterlight)
  (CallFunction|SetNewVisibility _winterlight))

(fn ConstructionScript
  (bind _staticmeshcomponent (Variables|Debug|GetStaticMeshComponent))
  (Utilities|IsValid _staticmeshcomponent
    (:Is%20Valid
      (Rendering|SetVisibility _staticmeshcomponent (Variables|Default|GetDebug) false))))

(fn Hide
  (params (IsHide :type Boolean))
  (Development|SetHiddeninGame (Variables|Debug|GetStaticMeshComponent) IsHide false)
  (Rendering|SetVisibility (Variables|Debug|GetStaticMeshComponent) (not IsHide) false))

(fn SetNewVisibility
  (params (bNewVisibility :type Boolean))
  (bind _staticmeshcomponent (Variables|Debug|GetStaticMeshComponent))
  (Utilities|IsValid _staticmeshcomponent
    (:Is%20Valid
      (if (not (Variables|Default|GetFreeze))
        (Rendering|SetVisibility _staticmeshcomponent bNewVisibility false)))))