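; BP_Fog is a fog actor that adapts the level's exponential height fog to the day-night cycle.
; NightIsComing switches the fog inscattering color between night and day colors, and the construction script applies the same choice from its IsNight flag.
; SetDayTime samples a density curve at the given time to drive fog density.
; Nodes adjusting height falloff and max opacity are present but disconnected.
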(event Custom|Night
  ;[1 1 1] Night
  (Class|ExponentialHeightFogComponent|SetFogInscatteringColor (Variables|Default|GetExponentialHeightFog) (Variables|Default|GetNightColor)))

(event Custom|Day
  ;[1 1 1] Day
  (Class|ExponentialHeightFogComponent|SetFogInscatteringColor (Variables|Default|GetExponentialHeightFog) (Variables|Default|GetDayColor)))

(event EventBeginPlay)

(event Collision|EventActorBeginOverlap
  (params (OtherActor :type Actor%20Object%20Reference)))

(event EventTick
  (params (DeltaSeconds :type Float%20%28single-precision%29)))

(event EventNightIsComing
  (params (IsNight :type Boolean))
  (if IsNight
    (CallFunction|Night)
    (else
      (CallFunction|Day))))

(event EventSetDayTime
  (params (Time :type Float%20%28single-precision%29))
  (Class|ExponentialHeightFogComponent|SetFogDensity (Variables|Default|GetExponentialHeightFog) (Math|Curves|GetFloatValue (Variables|Default|GetcurveDensityFog) Time)))

(fn ConstructionScript
  (if (Variables|Default|GetIsNight)
    (CallFunction|Night)
    (else
      (CallFunction|Day))))