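; BP_LightHouse is a night illumination actor that shows a static mesh only at night.
; The mesh is hidden on BeginPlay, and the NightIsComing event sets its visibility from the IsNight flag.
; The construction script applies an optional Mesh asset and uses the Debug flag to preview visibility in the editor.
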(event EventBeginPlay
  (Rendering|SetVisibility (Variables|Default|GetStaticMesh) false false))

(event Collision|EventActorBeginOverlap
  (params (OtherActor :type Actor%20Object%20Reference)))

(event EventTick
  (params (DeltaSeconds :type Float%20%28single-precision%29)))

(event EventNightIsComing
  (params (IsNight :type Boolean))
  (Rendering|SetVisibility (Variables|Default|GetStaticMesh) IsNight false))

(fn ConstructionScript
  (bind _mesh (Variables|Default|GetMesh))
  (Rendering|SetVisibility (Variables|Default|GetStaticMesh) (Variables|Default|GetDebug) false)
  (Utilities|IsValid _mesh
    (:Is%20Valid
      (Components|StaticMesh|SetStaticMesh (Variables|Default|GetStaticMesh) _mesh))))