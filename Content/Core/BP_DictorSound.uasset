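; Audio manager for background music and narrator (dictor) voice-overs, using 2D UI sounds.
; On BeginPlay it creates general and panorama tracks, and SetNewState swaps them, with only the Panorama state using the panorama track.
; Play and pause helpers check ArchGameMode flags, though pausing tests the voice flag rather than sound.
; House narration plays once per key via map lookups; DictorVoicePlay and StopGeneral are empty stubs.
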(event Custom|StopGeneral
  ;[1 1 1] Stop
)

(event EventBeginPlay
  ;[1 1 1] Start
  (bind _gamemode (CallFunction|GetArchGameMode))
  (Variables|Default|SetGame%20Mode _gamemode)
  (if (Variables|Default|GetIsAudioOn)
    (CallFunction|CreateMusic)
    (CallFunction|PlayMusic (Variables|Default|GetGeneralAudio))))

(event EventMusicAudioPlay
  (params (Play :type Boolean))
  ;[1 1 1] BackMusic
  (if (Variables|Default|GetIsAudioOn)
    (if Play
      (CallFunction|PlayMusic (Variables|Default|GetGeneralAudio))
      (else
        (CallFunction|PauseMusic (Variables|Default|GetGeneralAudio))
        (CallFunction|PauseMusic (Variables|Default|GetPanoramaAudio))))))

(event EventDictorVoicePlay
  (params (Enable :type Boolean))
  ;[1 1 1] Stop
  (if Enable
    _))

(event EventSetNewState
  (params (NewState :type E_TrainState%20Enum :default "NewEnumerator0") (SectionSelect :type BP%20Touch%20Vagon%20Object%20Reference) (FlatSelect :type BP%20Touch%20Coupe%20Object%20Reference) (SelectGroup :type Integer) (IsChange :type Boolean))
  ;[1 1 1] Comment
  (if (Variables|Default|GetIsAudioOn)
    (switch Utilities|FlowControl|Switch|SwitchonE_TrainState NewState
      (:NewEnumerator0
        (CallFunction|PauseMusic (Variables|Default|GetPanoramaAudio) :!label _label)
        (CallFunction|PlayMusic (Variables|Default|GetGeneralAudio)))
      (:NewEnumerator2
        (goto _label))
      (:NewEnumerator1
        (goto _label))
      (:NewEnumerator3
        (CallFunction|PauseMusic (Variables|Default|GetGeneralAudio))
        (CallFunction|PlayMusic (Variables|Default|GetPanoramaAudio)))
      (:NewEnumerator5
        (goto _label))
      (:NewEnumerator4
        (goto _label)))))

(fn ConstructionScript)

(fn CreateHouseAudio
  (params (InputPin :type Integer))
  (bind _dictorhousemap (Variables|Audio|GetDictorHouseMap))
  (bind (_value _returnvalue) (Utilities|Map|Find _dictorhousemap InputPin))
  (if (not (Variables|Default|GetIsPlayHouseDictor))
    (if _returnvalue
      (bind _returnvalue_2 (Audio|CreateSound2D _value 1.0 1.0 0.0 0))
      (bind _output_get (Variables|Default|SetDictorHouse2D _returnvalue_2))
      (Audio|Components|Audio|Play _output_get 0.0)
      (Variables|Default|SetIsPlayHouseDictor true)
      (Class|AudioComponent|SetUISound (Variables|Default|GetDictorHouse2D) true))))

(fn StartGeneralDictor
  (bind _returnvalue (Audio|CreateSound2D 0 1.0 1.0 0.0 0 false false))
  (bind _output_get (Variables|Default|SetDictorGeneral2D _returnvalue))
  (Audio|Components|Audio|FadeIn _output_get (Variables|Default|GetFadeDuration) 1.0 0.0 "Logarithmic" :!class /Script/Engine.AudioComponent)
  (Class|AudioComponent|SetUISound (Variables|Default|GetDictorGeneral2D) true))

(fn CreateMusic
  (Utilities|FlowControl|Sequence
    (:then_0
      (bind _returnvalue (Audio|CreateSound2D (Variables|Audio|GetAudioGeneral) 1.0 1.0 0.0 0 false false))
      (bind _output_get (Variables|Default|SetGeneralAudio _returnvalue))
      (Class|AudioComponent|SetUISound _output_get true))
    (:then_1
      (bind _returnvalue_2 (Audio|CreateSound2D (Variables|Audio|GetAudioPanorama) 1.0 1.0 0.0 0 false false))
      (bind _output_get_2 (Variables|Default|SetPanoramaAudio _returnvalue_2))
      (Class|AudioComponent|SetUISound _output_get_2 true))))

(fn PlayMusic
  (params (Audio :type Audio%20Component%20Object%20Reference))
  (if (and (Default|IsSoundEnable (Variables|Default|GetGame%20Mode)) (Utilities|IsValid Audio))
    (switch Utilities|FlowControl|Switch|SwitchonEAudioComponentPlayState (Audio|Components|Audio|GetPlayState Audio)
      (:Stopped
        _)
      (:Paused
        _))
    (Class|AudioComponent|SetPaused Audio false)
    (Audio|Components|Audio|FadeIn Audio (Variables|Default|GetFadeDuration) 1.0 0.0 "Linear" :!class /Script/Engine.AudioComponent)
    (Development|PrintString "Play")))

(fn PlayHouseGroupDictorAudio
  (params (InputPin :type Integer))
  (bind _oneplayhouseflag (Variables|Default|GetOnePlayHouseFlag))
  (bind _oneplayhouseflag_2 (Variables|Default|GetOnePlayHouseFlag))
  (bind (_value _returnvalue) (Utilities|Map|Find _oneplayhouseflag InputPin))
  (if (Default|IsVoiceEnable (Variables|Default|GetGame%20Mode))
    (if (and (not _value) _returnvalue)
      (CallFunction|CreateHouseAudio InputPin)
      (Utilities|Map|Remove _oneplayhouseflag_2 InputPin)
      (Utilities|Map|Add _oneplayhouseflag_2 InputPin true))))

(fn PauseMusic
  (params (Audio :type Audio%20Component%20Object%20Reference))
  (if (and (Default|IsVoiceEnable (Variables|Default|GetGame%20Mode)) (Utilities|IsValid Audio))
    (switch Utilities|FlowControl|Switch|SwitchonEAudioComponentPlayState (Audio|Components|Audio|GetPlayState Audio)
      (:Playing
        (Audio|Components|Audio|FadeOut Audio (Variables|Default|GetFadeDuration) 0.0 "Linear" :!class /Script/Engine.AudioComponent)
        (Class|AudioComponent|SetPaused Audio true)
        (Development|PrintString "Pause")))))

(fn StopHousePresent
  (bind _dictorhouse2d (Variables|Default|GetDictorHouse2D))
  (if (Variables|Default|GetIsPlayHouseDictor)
    (Utilities|IsValid _dictorhouse2d
      (:Is%20Valid
        (Audio|Components|Audio|FadeOut _dictorhouse2d 1.0 0.0 "Linear" :!class /Script/Engine.AudioComponent)
        (Variables|Default|SetIsPlayHouseDictor false)))))