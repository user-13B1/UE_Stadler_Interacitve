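; BP_AudioHouse is a sound hub that plays UI feedback for info widget toggles and state changes.
; BeginPlay adds three audio components, stored as InfoWidget, Close and ClickA.
; ShowInfoWidget plays InfoWidget on show and ClickA on hide, leaving Close unused in this graph.
; SetNewState switches over the view states (General, Vagon, Coupe, Panorama, Train) with no per-state logic, then plays ClickA.
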(event EventBeginPlay
  (bind _returnvalue (AddComponent|AddAudioComponent false))
  (Variables|Default|SetInfoWidget _returnvalue)
  (bind _returnvalue_2 (AddComponent|AddAudioComponent false))
  (Variables|Default|SetClose _returnvalue_2)
  (bind _returnvalue_3 (AddComponent|AddAudioComponent false))
  (Variables|Default|SetClick_A _returnvalue_3))

(event EventShowInfoWidget
  (params (Show :type Boolean) (Texture :type Array%20of%20Texture%202D%20Object%20References) (ShowInfoText :type Boolean) (Title1 :type Text) (Text1 :type Text) (Title2 :type Text) (Text2 :type Text) (Title3 :type Text) (Text3 :type Text))
  (if Show
    (Audio|Components|Audio|Play (Variables|Default|GetInfoWidget) 0.0)
    (else
      (Audio|Components|Audio|Play (Variables|Default|GetClick_A) 0.0))))

(event EventSetNewState
  (params (NewState :type E_TrainState%20Enum :default "NewEnumerator0") (SectionSelect :type BP%20Touch%20Vagon%20Object%20Reference) (FlatSelect :type BP%20Touch%20Coupe%20Object%20Reference) (SelectGroup :type Integer) (IsChange :type Boolean))
  (switch Utilities|FlowControl|Switch|SwitchonE_TrainState NewState
    (:NewEnumerator0
      _)
    (:NewEnumerator2
      _)
    (:NewEnumerator1
      _)
    (:NewEnumerator3
      _)
    (:NewEnumerator5
      _))
  (Audio|Components|Audio|Play (Variables|Default|GetClick_A) 0.0))

(fn ConstructionScript)