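; Building section actor for an architectural viewer, identified by house, part, section and floor.
; BeginPlay validates setup and optionally preloads its floor-plan interior as a hidden streamed level instance at the mesh's location.
; SetNewState drives visibility: flat selection hides higher floors in the same house part, reveals same-floor interiors and flags the matching section.
; Other states restore the mesh and close the interior; some states also swap the wall material.
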(event Custom|Hide
  ;[1 1 1] Hide
  (CallFunction|HideMesh))

(event Custom|Show
  ;[1 1 1] Show
  (CallFunction|ShowMesh))

(event Custom|StateSection
  (params (TouchSection :type BP%20Touch%20Vagon%20Object%20Reference))
  ;[1 1 1] Section
  (CallFunction|Show)
  (CallFunction|DeselectThisFlat)
  (CallFunction|CloseFloorPlanInterior))

(event Custom|StateGeneral
  ;[1 1 1] General
  (CallFunction|Show)
  (CallFunction|DeselectThisFlat)
  (CallFunction|CloseFloorPlanInterior))

(event Custom|StatePanorama
  ;[1 1 1] Panorama
  (CallFunction|Show)
  (CallFunction|DeselectThisFlat)
  (CallFunction|CloseFloorPlanInterior))

(event EventBeginPlay
  ;[1 1 1] START
  (CallFunction|UpdateInteriorMapRotater)
  (Variables|Default|SetThisFlat (Utilities|Struct|MakeST_HouseInfo (Variables|Default|GetHouse) (Variables|Default|GetSection) (Variables|Default|GetFloor) (Variables|Default|GetPart) 0))
  (bind _result (CallFunction|ValidateFloor))
  (if _result
    (CallFunction|PreLoadFloorPlan)
    (bind _gamemode (CallFunction|GetArchGameMode))
    (Variables|Default|SetArchGameMode _gamemode)
    (Collision|SetCollisionEnabled (Variables|Default|GetFlatMesh) "NoCollision")))

(event EventSetNewState
  (params (NewState :type E_TrainState%20Enum :default "NewEnumerator0") (SectionSelect :type BP%20Touch%20Vagon%20Object%20Reference) (FlatSelect :type BP%20Touch%20Coupe%20Object%20Reference) (SelectGroup :type Integer) (IsChange :type Boolean))
  ;[1 1 1] Select state
  (switch Utilities|FlowControl|Switch|SwitchonE_TrainState NewState
    (:NewEnumerator0
      (CallFunction|StateGeneral :!label _label)
      (Material|MaterialWallSetBlack))
    (:NewEnumerator2
      (CallFunction|StateSection SectionSelect)
      (Material|MaterialWallSetBlack))
    (:NewEnumerator1
      (CallFunction|SetStateSelectFlat FlatSelect)
      (Material|MaterialWallSetWhite))
    (:NewEnumerator3
      (CallFunction|StatePanorama))
    (:NewEnumerator5
      (goto _label))))

(event EventHideSection
  (params (IsHide :type Boolean) (Section :type Integer) (Group :type Integer))
  (bind _returnvalue (not IsHide))
  (bind _additmeshcomp (Variables|Additional|GetAdditMeshComp))
  ;[1 1 1] Comment
  (if (and (== Section (Variables|Default|GetPart)) (== Group (Variables|Default|GetHouse)))
    (Rendering|SetVisibility (Variables|Default|GetFlatMesh) _returnvalue true)
    (Utilities|IsValid _additmeshcomp
      (:Is%20Valid
        (Rendering|SetVisibility _additmeshcomp _returnvalue true)))))

(fn ConstructionScript
  (CallFunction|UpdateInteriorMapRotater)
  (CallFunction|UpdateSideBlock))

(fn SuitableforUp
  (params (SelectFloor :type Integer) (SelectSection :type Integer) (SelectHouse :type Integer))
  (return (Math|Boolean|ANDBoolean (> (Variables|Default|Getfloor) SelectFloor) (== SelectHouse (Variables|Default|Gethouse)) (Variables|Default|GetbIsDefaultPosition))))

(fn EqualFloor
  (params (Flat :type ST%20House%20Info%20Structure))
  (bind (_house _section _floor _part) (Utilities|Struct|BreakST_HouseInfo Flat))
  (return (Math|Boolean|ANDBoolean (== _floor (Variables|Default|GetFloor)) (== _section (Variables|Default|GetSection)) (== _part (Variables|Default|GetPart)) (== _house (Variables|Default|GetHouse)))))

(fn EqualforLoadFloorLevel
  (params (Flat :type ST%20House%20Info%20Structure))
  (bind (_house _section _floor _part) (Utilities|Struct|BreakST_HouseInfo Flat))
  (return (Math|Boolean|ANDBoolean (== _floor (Variables|Default|GetFloor)) (== _part (Variables|Default|GetPart)) (== _house (Variables|Default|GetHouse)))))

(fn UpdateInteriorMapRotater
  (if (Variables|Interior|GetIsRotateInterior)
    (Variables|Default|SetInteriorRotate (Transformation|GetWorldRotation (Variables|Default|GetFlatMesh)))
    (else
      (Variables|Default|SetInteriorRotate "0, 0, 0"))))

(fn LoadMap
  (params (InputPin :type World%20Soft%20Object%20Reference))
  (if (Utilities|IsValidSoftObjectReference InputPin)
    (bind (_boutsuccess _returnvalue) (Class|LevelStreamingDynamic|LoadLevelInstancebySoftObjectPtr InputPin (Transformation|GetWorldLocation (Variables|Default|GetFlatMesh)) (Variables|Default|GetInteriorRotate) "" 0 false))
    (if (Variables|Default|GetIsBlockOnLevelLoad)
      (Variables|/Script/Engine.LevelStreaming|SetbShouldBlockOnLoad _returnvalue true))
    (if _boutsuccess
      (return _returnvalue)
      (else
        (Development|PrintString "Error load floorplan")))))

(fn CheckandVisibleInteriorLevel
  (params (level :type Level%20Streaming%20Object%20Reference))
  (if (Utilities|IsValid level)
    (if (Variables|/Script/Engine.LevelStreaming|GetbShouldBeLoaded level)
      (Variables|/Script/Engine.LevelStreaming|SetbShouldBeVisible level true))))

(fn PreLoadFloorPlan
  (if (Variables|Default|GetLoadFloorPlan)
    (bind _returnvalue (CallFunction|LoadMap (Variables|Interior|GetFloorInterior)))
    (bind _output_get (Variables|Interior|SetInstanceFloorInterior _returnvalue))
    (Utilities|IsValid _output_get
      (:Is%20Valid
        (Variables|/Script/Engine.LevelStreaming|SetbShouldBeVisible _output_get false)))))

(fn ValidateFloor
  (bind _ballowedselect (Variables|Default|GetbAllowedSelect))
  (bind _floorinterior (Variables|Interior|GetFloorInterior))
  (bind _returnvalue (Utilities|IsValidSoftObjectReference _floorinterior))
  (bind _returnvalue_2 (Class|KismetMathLibrary|XORBoolean _returnvalue _ballowedselect))
  (bind _returnvalue_3 (not _returnvalue_2))
  (if _returnvalue_3
    _
    (else
      (Development|PrintString (Utilities|String|Append "Section not set. " (Utilities|String|ToString(Text) (Utilities|Text|ToText(Integer) (.section (Variables|Default|GetThisFlat))))))))
  (return _returnvalue_3))

(fn EqualPart
  (params (Flat :type ST%20House%20Info%20Structure))
  (bind (_house _section _floor _part) (Utilities|Struct|BreakST_HouseInfo Flat))
  (return (Math|Boolean|ANDBoolean (== _floor (Variables|Default|GetFloor)) (!= _section (Variables|Default|GetSection)) (== _part (Variables|Default|GetPart)) (== _house (Variables|Default|GetHouse)))))

(fn PreLoadBorder
  (params (Border :type Static%20Mesh%20Component%20Object%20Reference))
  (Utilities|IsValid Border
    (:Is%20Valid
      (Development|SetHiddeninGame Border true false)
      (Rendering|SetVisibility Border true false))))

(fn SetStateSelectFlat
  (params (SelectFlat :type BP%20Touch%20Coupe%20Object%20Reference))
  (Utilities|IsValid SelectFlat
    (:Is%20Valid
      (LocalVariables|SetFlat SelectFlat)
      (if (and (== (Variables|/Game/Core/BP_TouchCoupe.BP_TouchCoupe_C|GetVagon (LocalVariables|GetFlat)) (Variables|Default|GetHouse)) (== (Variables|Default|GetPart) (Variables|/Game/Core/BP_TouchCoupe.BP_TouchCoupe_C|GetTrain (LocalVariables|GetFlat))))
        (Utilities|FlowControl|Sequence
          (:then_0
            (if (== (Variables|Default|GetFloor) (Variables|/Game/Core/BP_TouchCoupe.BP_TouchCoupe_C|GetFloor (LocalVariables|GetFlat)))
              (CallFunction|OpenFloorPlanInterior)
              (Variables|Default|SetIsSelected (== (Variables|Default|GetSection) (Variables|/Game/Core/BP_TouchCoupe.BP_TouchCoupe_C|GetSection (LocalVariables|GetFlat))))
              (else
                (CallFunction|CloseFloorPlanInterior)
                (CallFunction|DeselectThisFlat))))
          (:then_1
            (if (> (Variables|Default|GetFloor) (Variables|/Game/Core/BP_TouchCoupe.BP_TouchCoupe_C|GetFloor (LocalVariables|GetFlat)))
              (CallFunction|Hide)
              (else
                (CallFunction|Show)))))
        (else
          (CallFunction|DeselectThisFlat)
          (CallFunction|CloseFloorPlanInterior)
          (CallFunction|Show)
          (return))))
    (:Is%20Not%20Valid
      (return))))

(fn DeselectThisFlat
  (if (Variables|Default|GetIsSelected)
    (Variables|Default|SetIsSelected false)))

(fn OpenFloorPlanInterior
  (if (not (Variables|Default|GetIsOpen))
    (Variables|Default|SetIsOpen true)
    (if (Utilities|IsValid (Variables|Interior|GetInstanceFloorInterior))
      (CallFunction|CheckandVisibleInteriorLevel (Variables|Interior|GetInstanceFloorInterior))
      (else
        (Development|PrintString "Not level to load")))))

(fn CloseFloorPlanInterior
  (if (Variables|Default|GetIsOpen)
    (Variables|Default|SetIsOpen false)
    (if (Utilities|IsValid (Variables|Interior|GetInstanceFloorInterior))
      (Variables|/Script/Engine.LevelStreaming|SetbShouldBeVisible (Variables|Interior|GetInstanceFloorInterior) false))))

(fn UpdateSideBlock
  (if (Utilities|IsValid (Variables|Additional|GetAdditMesh))
    (bind _returnvalue (AddComponent|AddStaticMeshComponent false))
    (bind _output_get (Variables|Additional|SetAdditMeshComp _returnvalue))
    (Components|StaticMesh|SetStaticMesh _output_get (Variables|Additional|GetAdditMesh))
    (Collision|SetCollisionEnabled _output_get "NoCollision")))

(fn ShowMesh
  (bind _additmeshcomp (Variables|Additional|GetAdditMeshComp))
  (if (Variables|Default|GetIsHide)
    (Variables|Default|SetIsHide false)
    (Utilities|FlowControl|Sequence
      (:then_0
        (Development|SetHiddeninGame (Variables|Default|GetFlatMesh) false false))
      (:then_1
        (Utilities|IsValid _additmeshcomp
          (:Is%20Valid
            (Development|SetHiddeninGame _additmeshcomp false false)))))))

(fn HideMesh
  (bind _additmeshcomp (Variables|Additional|GetAdditMeshComp))
  (if (not (Variables|Default|GetIsHide))
    (Variables|Default|SetIsHide true)
    (Utilities|FlowControl|Sequence
      (:then_0
        (Development|SetHiddeninGame (Variables|Default|GetFlatMesh) true false))
      (:then_1
        (Utilities|IsValid _additmeshcomp
          (:Is%20Valid
            (Development|SetHiddeninGame _additmeshcomp true false)))))))

(fn SetMaterial
  (params (Mesh :type Mesh%20Component%20Object%20Reference) (MaterialSlotName :type Name) (Material :type Material%20Interface%20Object%20Reference))
  (Utilities|IsValid Mesh
    (:Is%20Valid
      (if (Class|MeshComponent|IsMaterialSlotNameValid Mesh MaterialSlotName)
        (Rendering|Material|SetMaterialbyName Mesh MaterialSlotName Material)))))

(fn MaterialWallSetBlack
  (bind _whitematname (LocalVariables|GetWhiteMatName))
  (bind _materialblack (LocalVariables|GetMaterialBlack))
  (Utilities|FlowControl|Sequence
    (:then_0
      (Material|SetMaterial (Variables|Default|GetFlatMesh) _whitematname _materialblack))
    (:then_1
      (Material|SetMaterial (Variables|Additional|GetAdditMeshComp) _whitematname _materialblack))))

(fn MaterialWallSetWhite
  (bind _whitematname (LocalVariables|GetWhiteMatName))
  (Utilities|FlowControl|Sequence
    (:then_0
      (Material|SetMaterial (Variables|Default|GetFlatMesh) _whitematname))
    (:then_1
      (Material|SetMaterial (Variables|Additional|GetAdditMeshComp) _whitematname))))