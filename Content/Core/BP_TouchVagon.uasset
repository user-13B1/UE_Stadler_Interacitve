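; Invisible touch proxy for a train wagon that selects it on a double tap, detected with timed flags.
; A valid tap passes the object size to ArchGameMode and broadcasts the Vagon state.
; Incoming state changes toggle collision and selection, so the selected wagon stops taking touches.
; Mesh overlaps send hide/show messages for its Train and Vagon to all scene-state interface actors; Debug makes the proxy visible.
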(event OnInputTouchBegin(Mesh)
  (params (FingerIndex :type ETouchIndex%20Enum :default "Touch1") (TouchedComponent :type Primitive%20Component%20Object%20Reference))
  ;[1 1 1] Touch
  (switch Utilities|FlowControl|Switch|SwitchonETouchIndex FingerIndex
    (:Touch1
      (if (and (Variables|Flag|GetSuitableToTouch) (not (Variables|Flag|GetIsSelected)))
        (if (not (Variables|Flag|GetIsTouchOne))
          (Variables|Default|SetButtonDribbleBlock true)
          (Variables|Flag|SetIsTouchOne true)
          (Utilities|FlowControl|Delay 0.5)
          (Variables|Flag|SetIsTouchOne false)
          (elif (and (not (Variables|Flag|GetIsTouchTwo)) (not (Variables|Default|GetButtonDribbleBlock)))
            (Variables|Flag|SetIsTouchTwo true)
            (Utilities|FlowControl|Delay 0.2)
            (Variables|Flag|SetIsTouchTwo false)))))
    (:Touch2
      (Development|PrintString "Touch two fingre. " :!label _label))
    (:Touch3
      (goto _label))))

(event OnInputTouchEnd(Mesh)
  (params (FingerIndex :type ETouchIndex%20Enum :default "Touch1") (TouchedComponent :type Primitive%20Component%20Object%20Reference))
  ;[1 1 1] Touch
  (if (and (Variables|Flag|GetIsTouchOne) (not (Variables|Flag|GetIsTouchTwo)))
    (Utilities|FlowControl|Delay 0.05)
    (Variables|Default|SetButtonDribbleBlock false)
    (elif (Math|Boolean|ANDBoolean (Variables|Flag|GetIsTouchTwo) (Variables|Flag|GetSuitableToTouch) (Default|IsFree (Variables|Links|GetArchGameMode)))
      (Default|SetSizeCurrentObject (Variables|Links|GetArchGameMode) (Variables|Default|GetSizeObject))
      (CallFunction|SendAllNewState "NewEnumerator2" self))))

(event OnComponentBeginOverlap(Mesh)
  (params (OverlappedComponent :type Primitive%20Component%20Object%20Reference) (OtherActor :type Actor%20Object%20Reference) (OtherComp :type Primitive%20Component%20Object%20Reference) (OtherBodyIndex :type Integer) (bFromSweep :type Boolean) (SweepResult :type Hit%20Result%20Structure%20%28by%20ref%29))
  (CallFunction|HideHouseSection true))

(event OnComponentEndOverlap(Mesh)
  (params (OverlappedComponent :type Primitive%20Component%20Object%20Reference) (OtherActor :type Actor%20Object%20Reference) (OtherComp :type Primitive%20Component%20Object%20Reference) (OtherBodyIndex :type Integer))
  (CallFunction|HideHouseSection false))

(event Custom|StateSityMap
  ;[1 1 1] Comment
  (CallFunction|HideTouch)
  (Variables|Flag|SetIsSelected false))

(event Custom|StateGeneral
  ;[1 1 1] Comment
  (CallFunction|ShowTouch)
  (Variables|Flag|SetIsSelected false))

(event Custom|StateSection
  (params (Section :type BP%20Touch%20Vagon%20Object%20Reference))
  ;[1 1 1] Section
  (Utilities|IsValid Section
    (:Is%20Valid
      (if (and (== (Variables|Info|GetVagon) (Variables|BP_TouchVagon_C|GetVagon Section)) (== (Variables|Info|GetTrain) (Variables|BP_TouchVagon_C|GetTrain Section)))
        (CallFunction|HideTouch)
        (Variables|Flag|SetIsSelected true)
        (elif (Variables|Flag|GetIsSelected)
          (CallFunction|ShowTouch)
          (Variables|Flag|SetIsSelected false))))))

(event Custom|StateFlat
  (params (Section :type BP%20Touch%20Coupe%20Object%20Reference))
  ;[1 1 1] Flat
  (Utilities|IsValid Section
    (:Is%20Valid
      (if (and (== (Variables|Info|GetVagon) (Variables|/Game/Core/BP_TouchCoupe.BP_TouchCoupe_C|GetVagon Section)) (== (Variables|Info|GetTrain) (Variables|/Game/Core/BP_TouchCoupe.BP_TouchCoupe_C|GetTrain Section)))
        (CallFunction|HideTouch)
        (Variables|Flag|SetIsSelected true)
        (elif (Variables|Flag|GetIsSelected)
          (CallFunction|ShowTouch)
          (Variables|Flag|SetIsSelected false))))))

(event Custom|StatePanorama
  ;[1 1 1] Panorama
  (Variables|Flag|SetIsSelected false))

(event EventBeginPlay
  ;[1 1 1] Start
  (CallFunction|StartSetting)
  (bind _gamemode (CallFunction|GetArchGameMode))
  (Variables|Links|SetArchGameMode _gamemode))

(event EventSetNewState
  (params (NewState :type E_TrainState%20Enum :default "NewEnumerator0") (SectionSelect :type BP%20Touch%20Vagon%20Object%20Reference) (FlatSelect :type BP%20Touch%20Coupe%20Object%20Reference) (SelectGroup :type Integer) (IsChange :type Boolean))
  ;[1 1 1] SetState
  (switch Utilities|FlowControl|Switch|SwitchonE_TrainState NewState
    (:NewEnumerator0
      (CallFunction|StateGeneral :!label _label))
    (:NewEnumerator2
      (CallFunction|StateSection SectionSelect))
    (:NewEnumerator1
      (CallFunction|StateFlat FlatSelect))
    (:NewEnumerator3
      (CallFunction|StatePanorama))
    (:NewEnumerator5
      (goto _label))))

(fn ConstructionScript
  (bind _mesh (Variables|Default|GetMesh))
  (bind _meshcollision (Variables|Default|GetMeshCollision))
  (bind _mesh_2 (Variables|Default|GetMesh))
  (bind _mesh_3 (Variables|Default|GetMesh))
  (Utilities|IsValid _meshcollision
    (:Is%20Valid
      (Components|StaticMesh|SetStaticMesh _mesh_3 _meshcollision)
      (Rendering|Material|SetMaterial _mesh_3 0 "/Game/Stadler/Materials/Effect/M_Kontur_NoSelect.M_Kontur_NoSelect")
      (Collision|SetCollisionEnabled (Variables|Default|GetMesh) "NoCollision")
      (if (Variables|Default|GetDebug)
        (Development|SetHiddeninGame _mesh_2 false false)
        (Rendering|SetVisibility _mesh_2 true false)
        (else
          (Development|SetHiddeninGame _mesh true false)
          (Rendering|SetVisibility _mesh false false))))
    (:Is%20Not%20Valid
      (Development|PrintString "ErrorTouchMesh" true true "(R=1.000000,G=0.032086,B=0.000000,A=1.000000)" 12.0))))

(fn StartSetting
  (if (Math|Boolean|NORBoolean (== (Variables|Info|GetVagon) 0) (== (Variables|Info|GetTrain) 0))
    (CallFunction|ShowTouch)
    (else
      (Development|PrintString "BP_TouchVagon - data not set." true true "(R=1.000000,G=0.000000,B=0.037674,A=1.000000)"))))

(fn ShowTouch
  (Collision|SetCollisionEnabled (Variables|Default|GetMesh) "QueryAndPhysics")
  (Variables|Flag|SetSuitableToTouch true)
  (if (Variables|Default|GetDebug)
    (Development|SetHiddeninGame (Variables|Default|GetMesh) false false)))

(fn HideTouch
  (Collision|SetCollisionEnabled (Variables|Default|GetMesh) "NoCollision")
  (Variables|Flag|SetSuitableToTouch false)
  (if (Variables|Default|GetDebug)
    (Development|SetHiddeninGame (Variables|Default|GetMesh) true false)))

(fn HideHouseSection
  (params (IsHide :type Boolean))
  (if (> (Variables|Info|GetVagon) 0)
    (bind _outactors (Actor|GetAllActorswithInterface "/Game/Core/VIR_ScenaState_Interface.VIR_ScenaState_Interface_C"))
    (for _array_element _outactors
      (Class|VIRScenaStateInterface|HideSection(Message) _array_element IsHide (Variables|Info|GetTrain) (Variables|Info|GetVagon)))))