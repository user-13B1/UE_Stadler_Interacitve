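; BP_Sound is the background music manager, switching between a general track and a panorama track as the app state changes.
; On BeginPlay it creates both as persistent UI sounds and starts the general one.
; SetNewState selects panorama music only for the Panorama state, while MusicAudioPlay toggles music playback.
; Helpers fade and pause by play state, with playing gated on the game mode's sound flag but pausing on its voice flag.
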(event EventBeginPlay
  ;[1 1 1] Start
  (bind _gamemode (CallFunction|GetArchGameMode))
  (Variables|Default|SetGame%20Mode _gamemode)
  (if (Variables|Default|GetIsAudioOn)
    (CallFunction|CreateMusic)
    (CallFunction|PlayMusic (Variables|Default|GetGeneralAudio))))

(event EventMusicAudioPlay
  (params (Play :type Boolean))
  ;[1 1 1] BackMusic
  (if (Variables|Default|GetIsAudioOn)
    (if Play
      (CallFunction|PlayMusic (Variables|Default|GetGeneralAudio))
      (else
        (CallFunction|PauseMusic (Variables|Default|GetGeneralAudio))
        (CallFunction|PauseMusic (Variables|Default|GetPanoramaAudio))))))

(event EventSetNewState
  (params (NewState :type E_TrainState%20Enum :default "NewEnumerator0") (SectionSelect :type BP%20Touch%20Vagon%20Object%20Reference) (FlatSelect :type BP%20Touch%20Coupe%20Object%20Reference) (SelectGroup :type Integer) (IsChange :type Boolean))
  ;[1 1 1] Comment
  (if (Variables|Default|GetIsAudioOn)
    (switch Utilities|FlowControl|Switch|SwitchonE_TrainState NewState
      (:NewEnumerator0
        (CallFunction|PauseMusic (Variables|Default|GetPanoramaAudio) :!label _label)
        (CallFunction|PlayMusic (Variables|Default|GetGeneralAudio)))
      (:NewEnumerator2
        (goto _label))
      (:NewEnumerator1
        (goto _label))
      (:NewEnumerator3
        (CallFunction|PauseMusic (Variables|Default|GetGeneralAudio))
        (CallFunction|PlayMusic (Variables|Default|GetPanoramaAudio)))
      (:NewEnumerator5
        (goto _label))
      (:NewEnumerator4
        (goto _label)))))

(fn ConstructionScript)

(fn CreateMusic
  (Utilities|FlowControl|Sequence
    (:then_0
      (bind _returnvalue (Audio|CreateSound2D (Variables|Audio|GetAudioGeneral) (Variables|Default|GetVolume%20Multiplier) 1.0 0.0 0 false false))
      (bind _output_get (Variables|Default|SetGeneralAudio _returnvalue))
      (Class|AudioComponent|SetUISound _output_get true))
    (:then_1
      (bind _returnvalue_2 (Audio|CreateSound2D (Variables|Audio|GetAudioPanorama) (Variables|Default|GetVolume%20Multiplier) 1.0 0.0 0 false false))
      (bind _output_get_2 (Variables|Default|SetPanoramaAudio _returnvalue_2))
      (Class|AudioComponent|SetUISound _output_get_2 true))))

(fn PlayMusic
  (params (Audio :type Audio%20Component%20Object%20Reference))
  (if (Math|Boolean|ANDBoolean (Default|IsSoundEnable (Variables|Default|GetGame%20Mode)) (Utilities|IsValid Audio) (Variables|Default|GetIsAudioOn))
    (switch Utilities|FlowControl|Switch|SwitchonEAudioComponentPlayState (Audio|Components|Audio|GetPlayState Audio)
      (:Stopped
        _)
      (:Paused
        _))
    (Class|AudioComponent|SetPaused Audio false)
    (Audio|Components|Audio|FadeIn Audio (Variables|Default|GetFadeDuration) 1.0 0.0 "Linear" :!class /Script/Engine.AudioComponent)))

(fn PauseMusic
  (params (Audio :type Audio%20Component%20Object%20Reference))
  (if (and (Default|IsVoiceEnable (Variables|Default|GetGame%20Mode)) (Utilities|IsValid Audio))
    (switch Utilities|FlowControl|Switch|SwitchonEAudioComponentPlayState (Audio|Components|Audio|GetPlayState Audio)
      (:Playing
        (Audio|Components|Audio|FadeOut Audio (Variables|Default|GetFadeDuration) 0.1 "Linear" :!class /Script/Engine.AudioComponent)
        (Class|AudioComponent|SetPaused Audio true)))))