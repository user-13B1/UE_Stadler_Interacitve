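; BP_PanoramaPawn is a pawn for looking around a panorama by rotating its camera.
; MoveUp, MoveRight and the combined MoveUpRight clamp their input, scale it and add it to the stored pitch and yaw, then set the camera's relative rotation with zero roll.
; Pitch is limited between angle bounds while yaw is unbounded, and both axes share PitchSpeed.
; The event graph holds no active logic.
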(event EventBeginPlay)

(event Collision|EventActorBeginOverlap
  (params (OtherActor :type Actor%20Object%20Reference)))

(event EventTick
  (params (DeltaSeconds :type Float%20%28single-precision%29)))

(fn ConstructionScript)

(fn MoveUp
  (params (Value :type Float%20%28single-precision%29))
  (bind _result (Math|Float|NegateFloat Value)
    (:%20%20
      (bind _output_get (Variables|Default|SetCurrPitch (Math|Float|ClampAngle (+ (* (Math|Float|Clamp(Float) _result -3.0 3.0) (Variables|Default|GetPitchSpeed)) (Variables|Default|GetCurrPitch)) (LocalVariables|GetMinAngelDegres) (LocalVariables|GetMaxAngelDegres))))
      (Transformation|SetRelativeRotation (Variables|Default|GetCamera) (Math|Rotator|MakeRotator 0.0 _output_get (Variables|Default|GetCurrYaw)) false false))))

(fn MoveRight
  (params (Value :type Float%20%28single-precision%29))
  (bind _output_get (Variables|Default|SetCurrYaw (+ (* (Math|Float|Clamp(Float) Value -3.0 3.0) (Variables|Default|GetPitchSpeed)) (Variables|Default|GetCurrYaw))))
  (Transformation|SetRelativeRotation (Variables|Default|GetCamera) (Math|Rotator|MakeRotator 0.0 (Variables|Default|GetCurrPitch) _output_get) false false))

(fn MoveUpRight
  (params (X :type Float%20%28single-precision%29) (Y :type Float%20%28single-precision%29))
  (bind _result (Math|Float|NegateFloat Y)
    (:%20%20
      (Variables|Default|SetCurrPitch (Math|Float|ClampAngle (+ (* (Math|Float|Clamp(Float) _result -3.0 3.0) (Variables|Default|GetPitchSpeed)) (Variables|Default|GetCurrPitch)) (LocalVariables|GetMinAngelDegres) (LocalVariables|GetMaxAngelDegres)))
      (Variables|Default|SetCurrYaw (+ (* (Math|Float|Clamp(Float) X -3.0 3.0) (Variables|Default|GetPitchSpeed)) (Variables|Default|GetCurrYaw)))
      (Transformation|SetRelativeRotation (Variables|Default|GetCamera) (Math|Rotator|MakeRotator 0.0 (Variables|Default|GetCurrPitch) (Variables|Default|GetCurrYaw)) false false))))